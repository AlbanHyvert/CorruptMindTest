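; Interactable hiding spot that lets the first-person character hide and come back out with the Interact input.
; Box overlap caches the character, enables input and opens a gate; end overlap closes the gate but leaves input enabled.
; While the gate is open, Interact calls ToggleHide, which flips the character's visibility and collision and blends the camera between this actor and the character.
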(event OnComponentEndOverlap(Box)
  (params (OverlappedComponent :type Primitive%20Component%20Object%20Reference) (OtherActor :type Actor%20Object%20Reference) (OtherComp :type Primitive%20Component%20Object%20Reference) (OtherBodyIndex :type Integer))
  ;[1 1 1] Near Door Detection
  (Utilities|Casting|CastToFirstPersonCharacter OtherActor
    (:then
      (Input|EnableInput (Game|GetPlayerController 0))
      (Utilities|FlowControl|Gate true) ; enters at Close
    )
    (:CastFailed
      (Development|PrintString "Cast Failed"))))

(event OnComponentBeginOverlap(Box)
  (params (OverlappedComponent :type Primitive%20Component%20Object%20Reference) (OtherActor :type Actor%20Object%20Reference) (OtherComp :type Primitive%20Component%20Object%20Reference) (OtherBodyIndex :type Integer) (bFromSweep :type Boolean) (SweepResult :type Hit%20Result%20Structure%20%28by%20ref%29))
  ;[1 1 1] Near Door Detection
  (bind _asfirst_person_character (Utilities|Casting|CastToFirstPersonCharacter OtherActor)
    (:then
      (Variables|Default|SetChar%20REF _asfirst_person_character)
      (Input|EnableInput (Game|GetPlayerController 0))
      (Utilities|FlowControl|Gate true) ; enters at Open
    )
    (:CastFailed
      (Development|PrintString "Cast Failed"))))

(event Input|ActionEvents|InputActionInteract
  (params (Key :type Key%20Structure :default "None"))
  (:Pressed
    (Utilities|FlowControl|Gate true
      (:Exit
        (CallFunction|ToggleHide)))))

(fn ConstructionScript)

(fn ToggleHide
  (bind _returnvalue (Game|GetPlayerController 0))
  (bind _char_ref (Variables|Default|GetChar%20REF))
  (if (Variables|Default|GetIsHiding)
    (bind _output_get (Variables|Default|SetIsHiding false))
    (Rendering|SetActorHiddenInGame _char_ref _output_get)
    (Collision|SetActorEnableCollision _char_ref true)
    (Game|Player|SetViewTargetwithBlend _returnvalue _char_ref 0.6 "VTBlend_Linear" 0.0 false)
    (else
      (bind _output_get_2 (Variables|Default|SetIsHiding true))
      (Rendering|SetActorHiddenInGame _char_ref _output_get_2)
      (Collision|SetActorEnableCollision _char_ref false)
      (Game|Player|SetViewTargetwithBlend _returnvalue self 0.6 "VTBlend_Linear" 0.0 false))))